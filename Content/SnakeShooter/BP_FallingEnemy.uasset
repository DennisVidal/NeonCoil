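; Falling enemy Blueprint for the SnakeShooter game, handling the color-matched visual effects for its trail and death.
; On BeginPlay it copies the sprite's color into the trail effect's Color parameter.
; On death it spawns the death effect, if one is set, at the actor's transform and tints it with the same sprite color.
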(event `self.ReceiveBeginPlay`
  (`FXSystemComponent.SetColorParameter` (`self.TrailEffect`) "Color" (`PaperSpriteComponent.SpriteColor` (`self.SpriteComponent`))))

(event `self.OnDeath`
  (params (InKilledActor :type "Actor Object Reference") (InKiller :type "Actor Object Reference"))
  (bind _deatheffect (`self.DeathEffect`))
  (`/Engine/EditorBlueprintResources/StandardMacros.IsValid` _deatheffect
    (:`Is Valid`
      (bind _returnvalue (`NiagaraFunctionLibrary.SpawnSystemAtLocation` _deatheffect (`self.K2_GetActorLocation`) (`self.K2_GetActorRotation`) (`self.GetActorScale3D`)))
      (`/Engine/EditorBlueprintResources/StandardMacros.IsValid` _returnvalue
        (:`Is Valid`
          (`FXSystemComponent.SetColorParameter` _returnvalue "Color" (`PaperSpriteComponent.SpriteColor` (`self.SpriteComponent`))))))))

(fn `UserConstructionScript`
  (`parent.UserConstructionScript`))