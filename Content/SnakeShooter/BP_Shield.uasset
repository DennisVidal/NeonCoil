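; BP_Shield is a damageable shield actor in SnakeShooter, drawn with a Paper2D sprite and a ShieldEffect whose colors show remaining health.
; Both start at the full-health color, and on damage both are re-tinted by lerping between zero-health and full-health colors using normalized health.
; A bound death delegate spawns a Niagara break effect at the shield's transform, with fixed dimensions and the zero-health color.
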(event `self.ReceiveBeginPlay`
  (bind _fullhealthcolor (`self.FullHealthColor`))
  (`PaperSpriteComponent.SetSpriteColor` (`self.PaperSprite`) _fullhealthcolor)
  (`NiagaraComponent.SetVariableLinearColor` (`self.Shield Effect`) "Color" _fullhealthcolor)
  (add `self.OnDeathDelegate` (delegate `SpawnDeathEffect`)))

(event `SpawnDeathEffect` :!signature `self.OnDeathDelegate`
  (params (InKilledActor :type "Actor Object Reference") (InKiller :type "Actor Object Reference"))
  (bind _returnvalue (`NiagaraFunctionLibrary.SpawnSystemAtLocation` "/Game/SnakeShooter/Assets/Effects/NS_ShieldBreak.NS_ShieldBreak" (`self.K2_GetActorLocation`) (`self.K2_GetActorRotation`)))
  (`NiagaraComponent.SetVariableFloat` _returnvalue "Width" 3800.0)
  (`NiagaraComponent.SetVariableFloat` _returnvalue "Height" 255.0)
  (`NiagaraComponent.SetVariableLinearColor` _returnvalue "Color" (`self.ZeroHealthColor`)))

(event `self.OnDamaged`
  (params (InDamage :type "Float (single-precision)") (InDamagingActor :type "Actor Object Reference"))
  (bind _returnvalue (`KismetMathLibrary.LinearColorLerp` (`self.ZeroHealthColor`) (`self.FullHealthColor`) (`self.GetHealth01`)))
  (`PaperSpriteComponent.SetSpriteColor` (`self.PaperSprite`) _returnvalue)
  (`NiagaraComponent.SetVariableLinearColor` (`self.Shield Effect`) "Color" _returnvalue))

(fn `UserConstructionScript`)